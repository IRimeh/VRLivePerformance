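; Player spawn point actor that, when flagged to spawn the player on init, moves the existing player to its location at level start.
; On BeginPlay it gets the player from the custom game instance and calls a server teleport to its root's world position.
; If a TimelineController exists and the first one's level sequence is not playing, it then plays its audio from the start.
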(event EventBeginPlay
  (if (Variables|Default|GetSpawnPlayerHereOnInit)
    (bind _ascustom_game_instance (Utilities|Casting|CastToCustomGameInstance (Game|GetGameInstance)))
    (Utilities|IsValid (Variables|/Game/Blueprints/ProjectSettings/CustomGameInstance.CustomGameInstance_C|GetPlayer _ascustom_game_instance)
      (:Is%20Valid
        (Default|ServerTeleport (Variables|/Game/Blueprints/ProjectSettings/CustomGameInstance.CustomGameInstance_C|GetPlayer _ascustom_game_instance) (Transformation|GetWorldLocation (Variables|Default|GetDefaultSceneRoot)))
        (bind _outactors (Actor|GetAllActorsOfClass "/Game/Blueprints/Timeline/TimelineController.TimelineController_C"))
        (if (> (Utilities|Array|Length _outactors) 0)
          (if (not (Audio|Components|Audio|IsPlaying (Variables|/Script/LevelSequence.LevelSequenceActor|GetSequencePlayer (Variables|/Game/Blueprints/Timeline/TimelineController.TimelineController_C|GetLevelSequenceActor (Utilities|Array|Get(acopy) _outactors)))))
            (Audio|Components|Audio|Play (Variables|Default|GetAudio) 0.0)))))))

(event Collision|EventActorBeginOverlap
  (params (OtherActor :type Actor%20Object%20Reference)))

(event EventTick
  (params (DeltaSeconds :type Float%20%28single-precision%29)))

(fn ConstructionScript)