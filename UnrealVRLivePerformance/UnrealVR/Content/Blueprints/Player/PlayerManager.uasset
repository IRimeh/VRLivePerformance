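; PlayerManager actor that moves all VRPawn players together in a grid formation, with MoveAllPlayers meant to be called from the sequencer.
; It gathers the pawns on the server only and builds per-player offsets in a near-square grid, raised per row by HeightOffset.
; Spacing comes from a maximum formation size or a fixed value, or a custom offset list replaces the grid.
; Moves pass each pawn's offset, target and travel time to StartMovement.
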(event Custom|MoveAllPlayers
  (params (TargetLocation :type Vector) (TimeInSeconds :type Float%20%28single-precision%29))
  ;[1 1 1] Moves all the players and adds the offset (called from the sequencer)
  (CallFunction|GetAllPlayers)
  (for (_array_element _array_index) (Variables|Default|GetPlayers)
    (Default|StartMovement _array_element (Utilities|Array|Get(acopy) (Variables|Default|GetOffsetList) _array_index) TargetLocation TimeInSeconds)))

(event Custom|SetCustomOffset
  (params (OffsetList :type Array%20of%20Vectors))
  ;[1 1 1] Set completely customisble offset (doing this sucks though =D?)
  (Variables|Default|SetOffsetList OffsetList))

(event Custom|CalculateStandardOffset
  ;[1 1 1] Calculates standard movement offset, based on the OffSetValue and puts this in the list for each block
  (for (_ _array_index) (Variables|Default|GetPlayers)
    (Utilities|Array|SetArrayElem (Variables|Default|GetOffsetList) _array_index (Math|Vector|MakeVector (Math|Conversions|ToFloat(Integer) (- (* (+ (Math|Integer|%(Integer) _array_index (Variables|Default|GetColumns)) 1) (Variables|Default|GetOffSetValue)) (Variables|Default|GetHalfSize))) (Math|Conversions|ToFloat(Integer) (- (* (Math|Float|Ceil (/ (Math|Conversions|ToFloat(Integer) (+ _array_index 1)) (Math|Conversions|ToFloat(Integer) (Variables|Default|GetColumns)))) (Variables|Default|GetOffSetValue)) (Variables|Default|GetHalfSize))) (Math|Conversions|ToFloat(Integer) (* (Math|Float|Ceil (/ (Math|Conversions|ToFloat(Integer) (+ _array_index 1)) (Math|Conversions|ToFloat(Integer) (Variables|Default|GetColumns)))) (Variables|Default|GetHeightOffset)))) true)))

(event Custom|GetAllPlayers
  ;[1 1 1] Adds all the players in the experience (at the start)
  (if (Networking|IsServer)
    (bind _outactors (Actor|GetAllActorsOfClass "/Game/Blueprints/Player/VRPawn.VRPawn_C"))
    (Variables|Default|SetPlayers _outactors)))

(event Custom|SetOffSetIndividual
  (params (IndividualOffSet :type Integer))
  ;[1 1 1] Sets the offset, not taking in account of the maxsize.
  (Variables|Default|SetOffSetValue IndividualOffSet)
  (CallFunction|GetAllPlayers)
  (bind _output_get (Variables|Default|SetColumns (Math|Float|Ceil (Math|Float|Sqrt (Math|Conversions|ToFloat(Integer) (Utilities|Array|Length (Variables|Default|GetPlayers)))))))
  (Variables|Default|SetHalfSize (/ (+ (Variables|Default|GetOffSetValue) (* (Variables|Default|GetOffSetValue) _output_get)) 2))
  (CallFunction|CalculateStandardOffset))

(event Custom|SetOffsetFromMaxSize
  (params (MaxSize :type Integer))
  (bind _players (Variables|Default|GetPlayers))
  (bind _returnvalue (Utilities|Array|Length _players))
  ;[1 1 1] Sets the offset based on the maximum size in which all the players should fit.
  (Variables|Default|SetMaxSize MaxSize)
  (CallFunction|GetAllPlayers)
  (bind _output_get (Variables|Default|SetColumns (Math|Float|Ceil (Math|Float|Sqrt (Math|Conversions|ToFloat(Integer) _returnvalue)))))
  (if (> _returnvalue 1)
    (bind _output_get_2 (Variables|Default|SetOffSetValue (/ (Variables|Default|GetMaxSize) (- _output_get 1))))
    (Variables|Default|SetHalfSize (/ (+ _output_get_2 (* _output_get_2 _output_get)) 2)))
  (CallFunction|CalculateStandardOffset))

(event EventBeginPlay
  ;[1 1 1] Adds all the players in the experience (at the start)
  (if (Networking|IsServer)
    (bind _outactors (Actor|GetAllActorsOfClass "/Game/Blueprints/Player/VRPawn.VRPawn_C"))
    (Variables|Default|SetPlayers _outactors)))

(event Collision|EventActorBeginOverlap
  (params (OtherActor :type Actor%20Object%20Reference)))

(event EventTick
  (params (DeltaSeconds :type Float%20%28single-precision%29)))

(fn ConstructionScript)