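; Multiplayer game mode that spawns VR pawns for players and handles teleporting them to spawn locations.
; ChoosePlayerStart itself spawns and possesses a VRPawn, returning that pawn as the start.
; GetSpawnLocation picks a random actor tagged SpawnLocation, falling back to the world origin, with no occupancy check.
; Two helper functions teleport one player's pawn or all players' pawns, drawing a fresh random location for each.
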(event EventTick
  (params (DeltaSeconds :type Float%20%28single-precision%29)))

(fn ConstructionScript)

(fn ChoosePlayerStart
  (params (Player :type Controller%20Object%20Reference))
  ;[1 1 1] Spawn And Possess Pawn
  (bind _spawnlocation (CallFunction|GetSpawnLocation))
  (bind _returnvalue (Game|SpawnActorfromClass "/Game/Blueprints/Player/VRPawn.VRPawn_C" (Math|Transform|MakeTransform _spawnlocation) "AlwaysSpawn" 0 0))
  (Pawn|Possess Player _returnvalue)
  (return _returnvalue))

(fn GetSpawnLocation
  (bind _outactors (Actor|GetAllActorswithTag "SpawnLocation"))
  (if (> (Utilities|Array|Length _outactors) 0)
    (return (Transformation|GetActorLocation (Utilities|Array|Get(acopy) _outactors (Math|Random|RandomIntegerinRange 0 (- (Utilities|Array|Length _outactors) 1)))))
    (else
      (return "0, 0, 0"))))

(fn TeleportPlayerstoSpawnLocation
  (bind _returnvalue (Class|GameModeBase|GetNumPlayers (Game|GetGameMode)))
  (for _index (range 0 (- _returnvalue 1))
    (bind _spawnlocation (CallFunction|GetSpawnLocation))
    (Transformation|SetActorLocation (Pawn|GetControlledPawn (Game|GetPlayerController _index)) _spawnlocation false true)))

(fn TeleportPlayertoSpawnLocation
  (params (Player :type Controller%20Object%20Reference))
  (bind _spawnlocation (CallFunction|GetSpawnLocation))
  (Transformation|SetActorLocation (Pawn|GetControlledPawn Player) _spawnlocation false true))