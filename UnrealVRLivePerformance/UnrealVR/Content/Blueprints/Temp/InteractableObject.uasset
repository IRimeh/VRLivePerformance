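; InteractableObject is an actor that shows an outline when selected and opens the StageLevel map when interacted with.
; OnSelected plays the ShowOutline timeline to drive the OutlineThickness material parameter on the Outline component, while OnDeselected plays HideOutline, which sets it straight to zero.
; Both selection events print debug strings.
; OnInteract passes a hard-coded absolute local .umap file path to OpenLevelByName.
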(event EventBeginPlay)

(event Collision|EventActorBeginOverlap
  (params (OtherActor :type Actor%20Object%20Reference)))

(event EventTick
  (params (DeltaSeconds :type Float%20%28single-precision%29)))

(event EventOnInteract
  (Game|OpenLevel(byName) "C:/Users/454928/Documents/School/Year 4/SSS/Project/VRLivePerformance/UnrealVRLivePerformance/UnrealVR/Content/Maps/EnvironmentMaps/SkyscraperMap/StageLevel.umap"))

(event EventOnSelected
  (Development|PrintString "OnSelect" true true "(R=0.000000,G=0.000000,B=0.000000,A=1.000000)")
  (bind _time (Timeline|ShowOutline Play)
    (:Update
      (Rendering|Material|SetScalarParameterValueonMaterials (Variables|Default|GetOutline) "OutlineThickness" _time))))

(event EventOnDeselected
  (Development|PrintString "OnDeselect" true true "(R=0.000000,G=0.000000,B=0.000000,A=1.000000)")
  (Timeline|HideOutline Play
    (:Update
      (Rendering|Material|SetScalarParameterValueonMaterials (Variables|Default|GetOutline) "OutlineThickness" 0.0))))

(fn ConstructionScript)