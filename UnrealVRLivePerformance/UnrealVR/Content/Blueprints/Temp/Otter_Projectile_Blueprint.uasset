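; Otter projectile that launches along its mesh's forward vector on BeginPlay, then floats and swims by itself once below the water surface.
; Below the first found UIWSWaterBody's height, Tick applies depth-scaled buoyancy force and slowly levels rotation toward the flattened right vector.
; The right vector serves as swim heading: a debug-drawn line trace along it detects walls, yawing the mesh when blocked, otherwise pushing it onward.
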(event EventBeginPlay
  (bind _staticmeshcomponent (Variables|Debug|GetStaticMeshComponent))
  (bind _outactors (Actor|GetAllActorsOfClass "/Script/UIWS.UIWSWaterBody"))
  (Variables|Default|SetWater (Utilities|Array|Get(acopy) _outactors))
  (Physics|AddForce _staticmeshcomponent (* (Math|Vector|GetForwardVector _staticmeshcomponent) (Variables|Default|GetProjectileSpeed)) "None" false))

(event Collision|EventActorBeginOverlap
  (params (OtherActor :type Actor%20Object%20Reference)))

(event EventTick
  (params (DeltaSeconds :type Float%20%28single-precision%29))
  (bind _staticmeshcomponent (Variables|Debug|GetStaticMeshComponent))
  (bind _water (Variables|Default|GetWater))
  (bind _staticmeshcomponent_2 (Variables|Debug|GetStaticMeshComponent))
  (bind _staticmeshcomponent_3 (Variables|Debug|GetStaticMeshComponent))
  (bind _returnvalue (Transformation|GetWorldLocation _staticmeshcomponent))
  (bind _returnvalue_2 (Transformation|GetWorldLocation _staticmeshcomponent_2))
  (bind _rootcomponent (Variables|/Script/Engine.Actor|GetRootComponent _water))
  (bind _returnvalue_3 (Transformation|GetWorldLocation _rootcomponent))
  (if (< (.z _returnvalue_2) (.z _returnvalue_3))
    (Physics|AddForce (Variables|Debug|GetStaticMeshComponent) (Math|Vector|MakeVector 0.0 0.0 (* (Variables|Default|GetBoyancy) (Math|Float|Clamp(Float) (/ (Math|Float|Absolute(Float) (- (.z _returnvalue_2) (.z _returnvalue_3))) 2e+01)))) "None" false)
    (Transformation|SetWorldRotation _staticmeshcomponent (Math|Rotator|Lerp(Rotator) (Transformation|GetWorldRotation _staticmeshcomponent) (Math|Rotator|FindLookatRotation _returnvalue (+ _returnvalue (* (Math|Vector|GetRightVector _staticmeshcomponent) "1.000000,1.000000,0.000000"))) (* DeltaSeconds 0.01)) false false)
    (bind _returnvalue_4 (CallFunction|CheckifRunningIntoWall))
    (if _returnvalue_4
      (Transformation|AddWorldRotation (Variables|Debug|GetStaticMeshComponent) (Math|Rotator|MakeRotator 0.0 0.0 (Variables|Default|GetRotateSpeed)) false true)
      (else
        (Physics|AddForce _staticmeshcomponent_3 (* (Math|Vector|GetRightVector _staticmeshcomponent_3) (Variables|Default|GetMovementSpeed)) "None" false)))))

(fn ConstructionScript)

(fn CheckifRunningIntoWall
  (bind _staticmeshcomponent (Variables|Debug|GetStaticMeshComponent))
  (bind _returnvalue (Transformation|GetWorldLocation _staticmeshcomponent))
  (bind _returnvalue_2 (Collision|LineTraceForObjects _returnvalue (+ _returnvalue (* (Math|Vector|GetRightVector _staticmeshcomponent) 2e+02)) (Variables|Default|GetObjectTypes) false (Utilities|Array|MakeArray (Variables|Default|GetWater)) "ForOneFrame"))
  (return _returnvalue_2))