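; Otter actor that propels itself with physics force and turns away from obstacles in its path.
; Each tick it traces 200 units along the mesh's right vector, which serves as its forward direction, ignoring the Water actor and drawing the debug line.
; A hit yaws the mesh by a small fixed step; otherwise it adds force along that vector scaled by Speed.
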(event EventBeginPlay)

(event Collision|EventActorBeginOverlap
  (params (OtherActor :type Actor%20Object%20Reference)))

(event EventTick
  (params (DeltaSeconds :type Float%20%28single-precision%29))
  (bind _staticmeshcomponent (Variables|Debug|GetStaticMeshComponent))
  (bind _staticmeshcomponent_2 (Variables|Debug|GetStaticMeshComponent))
  (bind _returnvalue (Transformation|GetWorldLocation _staticmeshcomponent))
  (bind _returnvalue_2 (Collision|LineTraceForObjects _returnvalue (+ _returnvalue (* (Math|Vector|GetRightVector _staticmeshcomponent) 2e+02)) (Variables|Default|GetObjectTypes) false (Utilities|Array|MakeArray (Variables|Default|GetWater)) "ForOneFrame"))
  (if _returnvalue_2
    (Transformation|AddWorldRotation (Variables|Debug|GetStaticMeshComponent) (Math|Rotator|MakeRotator 0.0 0.0 5.0) false true)
    (else
      (Physics|AddForce _staticmeshcomponent_2 (* (Math|Vector|GetRightVector _staticmeshcomponent_2) (Variables|Default|GetSpeed)) "None" false))))

(fn ConstructionScript)