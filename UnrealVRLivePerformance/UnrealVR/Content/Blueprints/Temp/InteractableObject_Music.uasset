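; InteractableObject_Music is an interactable object that turns music on and off in the world.
; Each OnInteract call toggles its Audio component, activating it when silent and deactivating it when playing.
; An IsPlaying flag tracks the current state, and the object uses no tick or overlap logic.
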(event EventBeginPlay
  (|CallParentFunction) ; This node is disabled and will not be called.\nDrag off pins to build functionality.
)

(event Collision|EventActorBeginOverlap
  (params (OtherActor :type Actor%20Object%20Reference))
  (|CallParentFunction OtherActor) ; This node is disabled and will not be called.\nDrag off pins to build functionality.
)

(event EventTick
  (params (DeltaSeconds :type Float%20%28single-precision%29))
  (|CallParentFunction DeltaSeconds) ; This node is disabled and will not be called.\nDrag off pins to build functionality.
)

(event EventOnInteract
  (params (controller :type Static%20Mesh%20Component%20Object%20Reference))
  (bind _audio (Variables|Default|GetAudio))
  (if (Variables|Default|GetIsPlaying)
    (Components|Activation|Deactivate _audio)
    (Variables|Default|SetIsPlaying false)
    (else
      (Components|Activation|Activate _audio false)
      (Variables|Default|SetIsPlaying true))))

(fn ConstructionScript
  (|CallParentFunction))