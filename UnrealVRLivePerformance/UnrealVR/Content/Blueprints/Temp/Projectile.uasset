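; Simple physics projectile actor that launches itself on spawn and destroys itself on impact or timeout.
; BeginPlay applies a one-time, mass-dependent force along the mesh's forward vector, scaled by ProjectileSpeed, and binds the mesh's hit event to destruction.
; A GameplayTasks wait-delay task handles the lifetime timeout; hits apply no damage or effects.
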(event Custom|OnComponentHit_Event_0
  (params (HitComponent :type Primitive%20Component%20Object%20Reference) (OtherActor :type Actor%20Object%20Reference) (OtherComp :type Primitive%20Component%20Object%20Reference) (NormalImpulse :type Vector) (Hit :type Hit%20Result%20Structure%20%28by%20ref%29))
  (Actor|DestroyActor))

(event EventBeginPlay
  (Collision|AssignOnComponentHit (Variables|Components|GetMesh) (delegate Custom|OnComponentHit_Event_0))
  (Physics|AddForce (Variables|Components|GetMesh) (* (Math|Vector|GetForwardVector (Variables|Components|GetMesh)) (Variables|Default|GetProjectileSpeed)) "None" false)
  (GameplayTasks|TaskWaitDelay (Variables|Components|GetGameplayTasks) 1e+01
    (:OnFinish
      (Actor|DestroyActor))))

(fn ConstructionScript)