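; Timeline controller that plays a Level Sequence and appears meant to keep its playback in step between server and clients.
; BeginPlay creates an auto-playing sequence player with a configurable loop count, then scrubs it to the Time variable and plays.
; Each tick, the server writes playback position into Time, while non-servers re-scrub to Time and call Play again.
; Time also prints to screen every tick.
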(event EventBeginPlay
  (bind _outactor (Sequencer|Player|CreateLevelSequencePlayer (Variables|Timeline|GetLevelSequence) (Utilities|Struct|MakeMovieSceneSequencePlaybackSettings true (Utilities|Struct|MakeMovieSceneSequenceLoopCount (Variables|Timeline|GetLoopAmount)))))
  (Variables|Timeline|SetLevelSequenceActor _outactor)
  (CallFunction|StartPlaying))

(event EventTick
  (params (DeltaSeconds :type Float%20%28single-precision%29))
  (Development|PrintString (Utilities|String|ToString(Float) (Variables|Default|GetTime)) true true "(R=0.000000,G=0.660000,B=1.000000,A=1.000000)" 0.0)
  (if (Networking|IsServer)
    (Variables|Default|SetTime (Class|TimeManagementBlueprintLibrary|ToSeconds(QualifiedFrameTime) (Sequencer|Player|GetCurrentTime (Variables|/Script/LevelSequence.LevelSequenceActor|GetSequencePlayer (Variables|Timeline|GetLevelSequenceActor)))))
    (else
      (CallFunction|StartPlaying))))

(fn ConstructionScript)

(fn StartPlaying
  (bind _levelsequenceactor (Variables|Timeline|GetLevelSequenceActor))
  (bind _sequenceplayer (Variables|/Script/LevelSequence.LevelSequenceActor|GetSequencePlayer _levelsequenceactor))
  (Class|MovieSceneSequencePlayer|ScrubtoSeconds _sequenceplayer (Variables|Default|GetTime))
  (Sequencer|Player|Play _sequenceplayer :!class /Script/MovieScene.MovieSceneSequencePlayer))