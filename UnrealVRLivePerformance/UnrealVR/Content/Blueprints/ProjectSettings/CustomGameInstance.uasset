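; Custom game instance that manages the save slot, server connection, level switching and tutorial hooks for a stored non-dummy player.
; Init ensures a "Main" save exists; ServerConnect streams a transition level, joins a hardcoded IP, then applies the saved head preset.
; LoadLevel swaps streamed levels behind a transition widget using short delays, then teleports the player to the game mode's spawn.
; StartTutorial forwards to the player, while StopTutorial only prints a menu-reset message.
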(event Custom|ServerConnect
  (Game|LoadStreamLevel(byName) "Transition" true)
  (Utilities|FlowControl|Delay 0.2)
  (Class|NetworkingHelper|ConnecttoServer "192.168.178.157" (Game|GetPlayerController 0) false)
  (Utilities|FlowControl|Delay 2.0)
  (bind _returnvalue (SaveGame|LoadGamefromSlot "Main"))
  (bind _assave_state (Utilities|Casting|CastToSaveState _returnvalue))
  (Default|SetHeadPreset (Variables|Default|GetPlayer) (Variables|/Game/Blueprints/ProjectSettings/SaveState.SaveState_C|GetHeadCustomizationIndex _assave_state)))

(event Custom|LoadLevel
  (params (Level%20Name :type String) (Old%20Level%20Name :type String))
  (bind _returnvalue (UserInterface|CreateWidget "/Game/Maps/TransitionMapWidget.TransitionMapWidget_C"))
  (UserInterface|Viewport|AddtoViewport _returnvalue 0)
  (Utilities|FlowControl|Delay 0.1)
  (Game|UnloadStreamLevel(byName) (Utilities|String|StringToName Old%20Level%20Name) false)
  (Utilities|FlowControl|Delay 0.1)
  (Game|LoadStreamLevel(byName) (Utilities|String|StringToName Level%20Name) true)
  (Widget|RemovefromParent _returnvalue)
  (bind _asmultiplayer_game_mode (Utilities|Casting|CastToMultiplayerGameMode (Game|GetGameMode)))
  (bind _spawnlocation (Default|GetSpawnLocation _asmultiplayer_game_mode))
  (Transformation|SetActorLocation (Variables|Default|GetPlayer) _spawnlocation false true))

(event Custom|Start%20Tutorial
  (Default|StartTutorial (Variables|Default|GetPlayer)))

(event Custom|Stop%20Tutorial
  (Utilities|Casting|CastToBP_Menu_Left (Variables|/Script/Engine.ChildActorComponent|GetChildActor (Variables|/Game/Blueprints/VirtualReality/BP_MotionController.BP_MotionController_C|GetMenu (Variables|/Game/Blueprints/Player/VRPawn.VRPawn_C|GetLeftController (Variables|Default|GetPlayer)))))
  (Development|PrintString "RESET MENU"))

(event EventInit
  (bind _returnvalue (SaveGame|DoesSaveGameExist "Main"))
  (if _returnvalue
    (SaveGame|LoadGamefromSlot "Main")
    (else
      (bind _returnvalue_2 (SaveGame|CreateSaveGameObject "/Game/Blueprints/ProjectSettings/SaveState.SaveState_C"))
      (SaveGame|SaveGametoSlot _returnvalue_2 "Main"))))

(fn SetPlayer
  (params (Player :type VR%20Pawn%20Object%20Reference))
  (if (not (Variables|/Game/Blueprints/Player/VRPawn.VRPawn_C|GetIsDummy Player))
    (Variables|Default|SetPlayer Player)))