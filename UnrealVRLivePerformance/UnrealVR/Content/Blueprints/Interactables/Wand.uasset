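; BP interactable VR wand that can be grabbed from a distance and fires chargeable magic orbs.
; Interacting plays a timeline that lerps the mesh toward the motion controller's right grab origin.
; Using it while held toggles between charging, which grows the barrel on Tick up to a cap, and firing.
; Each shot replaces the previous orb, with charge setting scale and linear damping; firing or releasing resets the charge.
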(event Custom|Fire
  (params (ChargeSize :type Float%20%28single-precision%29))
  ;[1 1 1] Fires the orb
  (if (!= (Variables|Default|GetActiveOrb) 0)
    (Actor|DestroyActor (Variables|Default|GetActiveOrb)))
  (bind _returnvalue (Game|SpawnActorfromClass "/Game/Blueprints/Interactables/Wand_Extras/Orb.Orb_C" (Transformation|GetWorldTransform (Variables|Default|GetMagicBarrel)) "AlwaysSpawn" self 0))
  (Transformation|SetActorScale3D _returnvalue (* "3.000000,3.000000,3.000000" ChargeSize))
  (bind _output_get (Variables|Default|SetActiveOrb _returnvalue))
  (Class|PrimitiveComponent|SetLinearDamping (Variables|/Game/Blueprints/Interactables/Wand_Extras/Orb.Orb_C|GetBullet _output_get) ChargeSize)
  ;[1 1 1] Reset the wand
  (Variables|Default|SetChargeSize 0.1)
  (Transformation|SetRelativeScale3D (Variables|Default|GetMagicBarrel) "0.100000,0.100000,0.100000")
  (Variables|Default|SetCharging false))

(event EventOnInteractWhileHolding
  (params (controller :type Static%20Mesh%20Component%20Object%20Reference))
  ;[1 1 1] Fire
  (if (Variables|Default|GetCharging)
    (Variables|Default|SetCharging false)
    (Actor|Tick|SetActorTickEnabled false)
    (CallFunction|Fire (stale EventTick _output_get))
    (else
      (Variables|Default|SetCharging true)
      (Actor|Tick|SetActorTickEnabled true))))

(event EventTick
  (params (DeltaSeconds :type Float%20%28single-precision%29))
  ;[1 1 1] Fire
  (if (Variables|Default|GetCharging)
    (if (< (+ (Variables|Default|GetChargeSize) (* DeltaSeconds (Variables|Default|GetChargeSpeed))) 0.3)
      (bind _output_get (Variables|Default|SetChargeSize (+ (Variables|Default|GetChargeSize) (* DeltaSeconds (Variables|Default|GetChargeSpeed)))))
      (Transformation|SetRelativeScale3D (Variables|Default|GetMagicBarrel) (* "1.000000,1.000000,1.000000" _output_get))
      (else
        (Actor|Tick|SetActorTickEnabled false)))))

(event EventOnRelease
  ;[1 1 1] On releasing the interactable
  (Physics|SetSimulatePhysics (Variables|Character|GetMesh) true)
  ;[1 1 1] Reset the wand
  (Variables|Default|SetChargeSize 0.1)
  (Transformation|SetRelativeScale3D (Variables|Default|GetMagicBarrel) "0.100000,0.100000,0.100000")
  (Variables|Default|SetCharging false))

(event EventOnInteract
  (params (controller :type Static%20Mesh%20Component%20Object%20Reference))
  ;[1 1 1] Script that makes it grabbable from a distance
  (bind _asbp_motion_controller (Utilities|Casting|CastToBP_MotionController (Components|GetOwner controller)))
  (Variables|Default|SetController _asbp_motion_controller)
  (Physics|SetSimulatePhysics (Variables|Character|GetMesh) true)
  (bind _time (Timeline|MoveToController PlayFromStart)
    (:Update
      (Transformation|SetWorldLocation (Variables|Character|GetMesh) (Math|Vector|Lerp(Vector) (Transformation|GetWorldLocation (Variables|Default|GetHandle)) (Transformation|GetWorldLocation (Variables|/Game/Blueprints/VirtualReality/BP_MotionController.BP_MotionController_C|GetRightGrabOrigin (Variables|Default|GetController))) _time) false false))))

(fn ConstructionScript)