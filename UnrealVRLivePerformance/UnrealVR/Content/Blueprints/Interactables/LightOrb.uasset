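; LightOrb is a grabbable glowing orb that floats without gravity once released and slows to a stop.
; On BeginPlay it randomizes the point light color and the mesh material color with separate random vector evaluations.
; While not held, Tick damps linear velocity along a squared ease based on wall-clock time since release over SlowdownTime.
; A destroy event plays a timeline that drives light intensity and compounding mesh scale changes.
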(event Custom|onStartDestroying_1
  (bind _mesh (Variables|Character|GetMesh))
  (bind _val (Timeline|DestroyTimeline Play)
    (:Update
      (Rendering|Components|Light|SetIntensity (Variables|Default|GetPointLight) (+ 1e+04 (* 1e+04 _val)))
      (Transformation|SetWorldScale3D _mesh (* (Transformation|GetWorldScale _mesh) (- 1.01 _val))))))

(event EventBeginPlay
  (CallFunction|RandomizeColor))

(event Collision|EventActorBeginOverlap
  (params (OtherActor :type Actor%20Object%20Reference)))

(event EventOnRelease
  (Variables|Default|SetReleasedTime (Class|KismetMathLibrary|GetTotalMilliseconds (TimeOfDay|GetTimeOfDay (Math|DateTime|Now) :!class /Script/Engine.KismetMathLibrary)))
  (Physics|SetEnableGravity (Variables|Character|GetMesh) false)
  (Variables|Default|SetIsBeingHeld_0 false))

(event EventOnGrab
  (Variables|Default|SetIsBeingHeld_0 true))

(event EventTick
  (params (DeltaSeconds :type Float%20%28single-precision%29))
  (if (not (Variables|Default|GetIsBeingHeld_0))
    (bind _returnvalue (Physics|GetPhysicsLinearVelocity (Variables|Character|GetMesh) "None"))
    (Physics|SetPhysicsLinearVelocity (Variables|Character|GetMesh) (* _returnvalue (- 1.0 (Math|Float|Power (Math|Float|Clamp(Float) (/ (- (Class|KismetMathLibrary|GetTotalMilliseconds (TimeOfDay|GetTimeOfDay (Math|DateTime|Now) :!class /Script/Engine.KismetMathLibrary)) (Variables|Default|GetReleasedTime)) (Variables|Default|GetSlowdownTime))) 2.0))) false "None")))

(fn ConstructionScript)

(fn RandomizeColor
  (bind _returnvalue (Math|Random|RandomUnitVector))
  (bind _returnvalue_2 (Math|Vector|VectorGetAbs _returnvalue))
  (Rendering|Components|Light|SetLightColor (Variables|Default|GetPointLight) (Math|Conversions|ToLinearColor(Vector) _returnvalue_2) false)
  (Rendering|Material|SetVectorParameterValueonMaterials (Variables|Character|GetMesh) "Color" _returnvalue_2))