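; Interactable camera actor that the motion controller can grab from a distance.
; On interact it stores the BP_MotionController, disables mesh physics and plays a timeline that lerps the mesh from the Camera component's location toward the controller's right grab origin, re-read each update.
; Release re-enables physics, while the hold-interact event and construction script are empty.
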(event EventTick
  (params (DeltaSeconds :type Float%20%28single-precision%29)))

(event EventOnInteract
  (params (controller :type Static%20Mesh%20Component%20Object%20Reference))
  ;[1 1 1] Script that makes it grabbable from a distance
  (bind _asbp_motion_controller (Utilities|Casting|CastToBP_MotionController (Components|GetOwner controller)))
  (Variables|Default|SetController _asbp_motion_controller)
  (Physics|SetSimulatePhysics (Variables|Character|GetMesh) false)
  (bind _time (Timeline|Timeline_0 PlayFromStart)
    (:Update
      (Transformation|SetWorldLocation (Variables|Character|GetMesh) (Math|Vector|Lerp(Vector) (Transformation|GetWorldLocation (Variables|Default|GetCamera)) (Transformation|GetWorldLocation (Variables|/Game/Blueprints/VirtualReality/BP_MotionController.BP_MotionController_C|GetRightGrabOrigin (Variables|Default|GetController))) _time) false false))))

(event EventOnInteractWhileHolding
  (params (controller :type Static%20Mesh%20Component%20Object%20Reference)))

(event EventOnRelease
  ;[1 1 1] Enabling physics again
  (Physics|SetSimulatePhysics (Variables|Character|GetMesh) true))

(fn ConstructionScript)