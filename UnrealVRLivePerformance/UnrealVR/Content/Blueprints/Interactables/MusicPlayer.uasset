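; Interactable music player that toggles on interaction, hovering and spinning while on and falling under physics while off.
; While on, Tick yaws the mesh and lerps it toward a sine bob around its start position, with a random phase offset.
; Each toggle switches physics, gravity and outline color, and fades a referenced AudioActor's volume between full and near-silent instead of stopping it.
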(event Custom|Rotate
  (params (DeltaTime :type Float%20%28single-precision%29))
  (Transformation|AddWorldRotation (Variables|Default|GetStaticMesh) (Math|Rotator|MakeRotator 0.0 0.0 (* DeltaTime 1e+02)) false false))

(event Custom|FloatUpAndDown
  (params (DeltaTime :type Float%20%28single-precision%29))
  (Transformation|SetWorldLocation (Variables|Default|GetStaticMesh) (Math|Vector|Lerp(Vector) (Transformation|GetWorldLocation (Variables|Default|GetStaticMesh)) (+ (Variables|Default|GetStartPosition) (Math|Vector|MakeVector 0.0 0.0 (* (Math|Trig|Sin(Degrees) (* (+ (Utilities|Time|GetGameTimeinSeconds) (Variables|Default|GetRandomOffset)) (Variables|Floating|GetFloatSpeed))) (Variables|Floating|GetFloatDistance)))) DeltaTime) false true))

(event EventBeginPlay
  (|CallParentFunction)
  (Variables|Default|SetStartPosition (Transformation|GetWorldLocation (Variables|Character|GetMesh)))
  (Rendering|Material|SetVectorParameterValueonMaterials (Variables|Default|GetOutline) "OutlineColor" (Math|Conversions|ToVector(LinearColor) (Math|Conversions|ToLinearColor(Color) (Variables|Colors|GetDisableColor))))
  (Variables|Default|SetRandomOffset (Math|Random|RandomFloatinRange 0.0 1e+04)))

(event Collision|EventActorBeginOverlap
  (params (OtherActor :type Actor%20Object%20Reference))
  (|CallParentFunction OtherActor) ; This node is disabled and will not be called.\nDrag off pins to build functionality.
)

(event EventTick
  (params (DeltaSeconds :type Float%20%28single-precision%29))
  (|CallParentFunction DeltaSeconds)
  (if (Variables|Default|GetTurnedOn)
    (CallFunction|Rotate DeltaSeconds)
    (CallFunction|FloatUpandDown DeltaSeconds)))

(event EventOnInteract
  (params (controller :type Static%20Mesh%20Component%20Object%20Reference))
  (bind _output_get (Variables|Default|SetTurnedOn (not (Variables|Default|GetTurnedOn))))
  (if _output_get
    (CallFunction|Turnon)
    (else
      (CallFunction|TurnOff))))

(fn ConstructionScript
  (|CallParentFunction))

(fn Turnon
  (bind _staticmesh (Variables|Default|GetStaticMesh))
  (Physics|SetSimulatePhysics _staticmesh false)
  (Physics|SetEnableGravity _staticmesh false)
  (Rendering|Material|SetVectorParameterValueonMaterials (Variables|Default|GetOutline) "OutlineColor" (Math|Conversions|ToVector(LinearColor) (Math|Conversions|ToLinearColor(Color) (Variables|Colors|GetDisableColor))))
  (CallFunction|UpdateAudio 1.0))

(fn TurnOff
  (bind _staticmesh (Variables|Default|GetStaticMesh))
  (Physics|SetSimulatePhysics _staticmesh true)
  (Physics|SetEnableGravity _staticmesh true)
  (Rendering|Material|SetVectorParameterValueonMaterials (Variables|Default|GetOutline) "OutlineColor" (Math|Conversions|ToVector(LinearColor) (Math|Conversions|ToLinearColor(Color) (Variables|Colors|GetEnableColor))))
  (CallFunction|UpdateAudio 0.001))

(fn UpdateAudio
  (params (VolumeMultiplier :type Float%20%28single-precision%29))
  (bind _audioactor (Variables|Default|GetAudioActor))
  (Utilities|IsValid _audioactor
    (:Is%20Valid
      (Audio|Components|Audio|AdjustVolume (Actor|GetComponentbyClass _audioactor "/Script/Engine.AudioComponent") 0.25 VolumeMultiplier "Linear" :!class /Script/Engine.AudioComponent))))