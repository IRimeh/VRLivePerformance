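; ChangeBodyButton is an interactable button that cycles the player's body preset forward or backward.
; On interact, the NextOrPrevious flag picks the next or previous preset.
; It applies the change to an ExampleVRPawn reference and then to the Player held by CustomGameInstance, reached through a cast.
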(event EventBeginPlay
  (|CallParentFunction) ; This node is disabled and will not be called.\nDrag off pins to build functionality.
)

(event Collision|EventActorBeginOverlap
  (params (OtherActor :type Actor%20Object%20Reference))
  (|CallParentFunction OtherActor) ; This node is disabled and will not be called.\nDrag off pins to build functionality.
)

(event EventTick
  (params (DeltaSeconds :type Float%20%28single-precision%29))
  (|CallParentFunction DeltaSeconds) ; This node is disabled and will not be called.\nDrag off pins to build functionality.
)

(event EventOnInteract
  (params (controller :type Static%20Mesh%20Component%20Object%20Reference))
  (if (Variables|Default|GetNextOrPrevious)
    (Default|NextBodyPreset (Variables|Default|GetExampleVRPawn))
    (bind _ascustom_game_instance (Utilities|Casting|CastToCustomGameInstance (Game|GetGameInstance)))
    (Default|NextBodyPreset (Variables|/Game/Blueprints/ProjectSettings/CustomGameInstance.CustomGameInstance_C|GetPlayer _ascustom_game_instance))
    (else
      (Default|PreviousBodyPreset (Variables|Default|GetExampleVRPawn))
      (bind _ascustom_game_instance_2 (Utilities|Casting|CastToCustomGameInstance (Game|GetGameInstance)))
      (Default|PreviousBodyPreset (Variables|/Game/Blueprints/ProjectSettings/CustomGameInstance.CustomGameInstance_C|GetPlayer _ascustom_game_instance_2)))))

(fn ConstructionScript
  (|CallParentFunction))