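; SinglePlayerButton is an interactable that sends the game into the EngineerGreybox level through the CustomGameInstance's LoadLevel.
; OnInteract triggers the load immediately.
; BeginPlay also runs the same load automatically after a two-second delay, so the level changes even without interaction.
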(event EventBeginPlay
  (|CallParentFunction)
  (Utilities|FlowControl|Delay 2.0)
  (bind _ascustom_game_instance (Utilities|Casting|CastToCustomGameInstance (Game|GetGameInstance)))
  (Default|LoadLevel _ascustom_game_instance "EngineerGreybox"))

(event Collision|EventActorBeginOverlap
  (params (OtherActor :type Actor%20Object%20Reference))
  (|CallParentFunction OtherActor) ; This node is disabled and will not be called.\nDrag off pins to build functionality.
)

(event EventTick
  (params (DeltaSeconds :type Float%20%28single-precision%29))
  (|CallParentFunction DeltaSeconds) ; This node is disabled and will not be called.\nDrag off pins to build functionality.
)

(event EventOnInteract
  (params (controller :type Static%20Mesh%20Component%20Object%20Reference))
  (bind _ascustom_game_instance (Utilities|Casting|CastToCustomGameInstance (Game|GetGameInstance)))
  (Default|LoadLevel _ascustom_game_instance "EngineerGreybox"))

(fn ConstructionScript
  (|CallParentFunction))