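; A grabbable VR lighter that the player can light or put out while holding it, and that can be pulled to the right hand from a distance.
; Toggling goes through the Player, and the replicated IsLighterOn's OnRep switches Fire collision and fades its material through timelines.
; Tick watches the cap detector, blocking ignition while the cap is closed and extinguishing the flame when it shuts.
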(event Custom|TurnLighterOff
  (Variables|Default|SetIsLighterOn false))

(event Custom|TurnLighterOn
  (Variables|Default|SetIsLighterOn true))

(event Custom|LighterOnOffTurning
  (bind _fire (Variables|Default|GetFire))
  (bind _fire_2 (Variables|Default|GetFire))
  (if (Variables|Default|GetIsLighterOn)
    (Collision|SetCollisionEnabled _fire_2 "QueryOnly")
    (Variables|/Script/Engine.PrimitiveComponent|SetbGenerateOverlapEvents _fire_2 true)
    (bind _time (Timeline|TurnLighterOnTimeline PlayFromStart)
      (:Update
        (Rendering|Material|SetScalarParameterValueonMaterials (Variables|Default|GetFire) "On" _time)))
    (else
      (Collision|SetCollisionEnabled _fire "NoCollision")
      (Variables|/Script/Engine.PrimitiveComponent|SetbGenerateOverlapEvents _fire false)
      (bind _time_2 (Timeline|TurnLighterOffTimeline PlayFromStart)
        (:Update
          (Rendering|Material|SetScalarParameterValueonMaterials (Variables|Default|GetFire) "On" _time_2))))))

(event EventBeginPlay
  (bind _fire (Variables|Default|GetFire))
  (Collision|SetCollisionEnabled _fire "NoCollision")
  (Variables|/Script/Engine.PrimitiveComponent|SetbGenerateOverlapEvents _fire false)
  (bind _ascustom_game_instance (Utilities|Casting|CastToCustomGameInstance (Game|GetGameInstance)))
  (Variables|Default|SetPlayer (Variables|/Game/Blueprints/ProjectSettings/CustomGameInstance.CustomGameInstance_C|GetPlayer _ascustom_game_instance)))

(event Collision|EventActorBeginOverlap
  (params (OtherActor :type Actor%20Object%20Reference)))

(event EventTick
  (params (DeltaSeconds :type Float%20%28single-precision%29))
  (bind _capclosedetector (Variables|Default|GetCapCloseDetector))
  (bind _lightercap (Variables|Default|GetLighterCap))
  (bind _outoverlappingcomponents (Class|PrimitiveComponent|GetOverlappingComponents _capclosedetector))
  (bind _returnvalue (Utilities|Array|ContainsItem _outoverlappingcomponents _lightercap))
  (if (Math|Boolean|NotEqual(Boolean) _returnvalue (Variables|Default|GetIsCapClosed))
    (Variables|Default|SetIsCapClosed _returnvalue)
    (if (and _returnvalue (Variables|Default|GetIsLighterOn))
      (Default|LighterOff (Variables|Default|GetPlayer) self))))

(event EventOnInteractWhileHolding
  (params (controller :type Static%20Mesh%20Component%20Object%20Reference))
  (if (Variables|Default|GetIsLighterOn)
    (Default|LighterOff (Variables|Default|GetPlayer) self)
    (elif (not (Variables|Default|GetIsCapClosed))
      (Default|Lighteron (Variables|Default|GetPlayer) self))))

(event EventOnInteract
  (params (controller :type Static%20Mesh%20Component%20Object%20Reference))
  ;[1 1 1] Script that makes it grabbable from a distance
  (bind _asbp_motion_controller (Utilities|Casting|CastToBP_MotionController (Components|GetOwner controller)))
  (Variables|Default|SetController _asbp_motion_controller)
  (Physics|SetSimulatePhysics (Variables|Character|GetMesh) true)
  (bind _time (Timeline|Timeline_0_0 PlayFromStart)
    (:Update
      (Transformation|SetWorldLocation (Variables|Character|GetMesh) (Math|Vector|Lerp(Vector) (Transformation|GetWorldLocation (Variables|Character|GetMesh)) (Transformation|GetWorldLocation (Variables|/Game/Blueprints/VirtualReality/BP_MotionController.BP_MotionController_C|GetRightGrabOrigin (Variables|Default|GetController))) _time) false false))))

(event EventOnGrab
  (|CallParentFunction)
  (bind _ascustom_game_instance (Utilities|Casting|CastToCustomGameInstance (Game|GetGameInstance)))
  (Actor|SetOwner (Variables|/Game/Blueprints/ProjectSettings/CustomGameInstance.CustomGameInstance_C|GetPlayer _ascustom_game_instance)))

(fn ConstructionScript)

(fn OnRepIsLighteron
  (CallFunction|LighteronOffTurning))