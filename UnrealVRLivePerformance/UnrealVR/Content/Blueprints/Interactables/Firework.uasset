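; Grabbable VR firework that can be pulled from a distance to the motion controller's right grab origin, then lit, launched and exploded.
; Tick checks sphere overlaps for "Fire"-tagged components and passes itself to the player's Firework call, with SetOffFireworkServerSide exposed to start ignition.
; Chained timelines animate the fuse material, push the physics mesh along its up vector, then trigger a random explosion effect before delayed destruction.
; Releasing it lit raises angular damping.
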(event Custom|SetOffFirework
  ;[1 1 1] Fuse
  (if (not (Variables|Default|GetIsFireworkSetOff))
    (Variables|Default|SetIsFireworkSetOff true)
    (bind _time (Timeline|FuseTime Play)
      (:Update
        (Rendering|Material|SetScalarParameterValueonMaterials (Variables|Character|GetMesh) "FuseTime" _time))
      (:Finished
        (CallFunction|Pewpew)))))

(event Custom|Pewpew
  (bind _mesh (Variables|Character|GetMesh))
  (Components|Activation|Activate (Variables|Default|GetTrail) false)
  (Timeline|FireworkLaunch Play
    (:Update
      (if (Physics|IsSimulatingPhysics (Variables|Character|GetMesh) "None")
        (Physics|AddForce _mesh (* (Math|Vector|GetUpVector _mesh) 2e+03) "None" false)))
    (:Finished
      (CallFunction|Boomer))))

(event Custom|Boomer
  (Class|NiagaraComponent|SetAsset (Variables|Default|GetExplosion) (Utilities|Array|Get(acopy) (Variables|Default|GetFireworkAssets) (Math|Random|RandomIntegerinRange 0 (- (Utilities|Array|Length (Variables|Default|GetFireworkAssets)) 1))))
  (CallFunction|HideFirework)
  (Physics|SetSimulatePhysics (Variables|Character|GetMesh) false)
  (Components|Activation|Activate (Variables|Default|GetExplosion) false)
  (Utilities|FlowControl|Delay 4.0)
  (CallFunction|DeleteFireworks))

(event Custom|Hide%20Firework
  (Components|Activation|Deactivate (Variables|Default|GetTrail))
  (Rendering|SetVisibility (Variables|Character|GetMesh) false false))

(event Custom|Delete%20Fireworks
  (params (PSystem :type Niagara%20Component%20Object%20Reference))
  (Class|Interactable|StartDestroying))

(event Custom|SetOffFireworkServerSide
  ;[1 1 1] Fuse
  (CallFunction|SetOffFirework))

(event EventBeginPlay
  (bind _ascustom_game_instance (Utilities|Casting|CastToCustomGameInstance (Game|GetGameInstance)))
  (Variables|Default|SetPlayer (Variables|/Game/Blueprints/ProjectSettings/CustomGameInstance.CustomGameInstance_C|GetPlayer _ascustom_game_instance)))

(event EventOnRelease
  (if (Variables|Default|GetIsFireworkSetOff)
    (Class|PrimitiveComponent|SetAngularDamping (Variables|Character|GetMesh) 5e+02)))

(event EventTick
  (params (DeltaSeconds :type Float%20%28single-precision%29))
  (bind _sphere (Variables|Default|GetSphere))
  (bind _outoverlappingcomponents (Class|PrimitiveComponent|GetOverlappingComponents _sphere))
  (if (not (Variables|Default|GetIsFireworkSetOff))
    ;[1 1 1] Lighter Firework Collision
    (if (> (Utilities|Array|Length _outoverlappingcomponents) 0)
      (for _array_element _outoverlappingcomponents
        (if (Components|ComponentHasTag _array_element "Fire")
          (Default|Firework (Variables|Default|GetPlayer) self))))))

(event EventOnInteract
  (params (controller :type Static%20Mesh%20Component%20Object%20Reference))
  ;[1 1 1] Script that makes it grabbable from a distance
  (bind _asbp_motion_controller (Utilities|Casting|CastToBP_MotionController (Components|GetOwner controller)))
  (Variables|Default|SetController _asbp_motion_controller)
  (Physics|SetSimulatePhysics (Variables|Character|GetMesh) true)
  (bind _time (Timeline|Timeline_0_0 PlayFromStart)
    (:Update
      (Transformation|SetWorldLocation (Variables|Character|GetMesh) (Math|Vector|Lerp(Vector) (Transformation|GetWorldLocation (Variables|Character|GetMesh)) (Transformation|GetWorldLocation (Variables|/Game/Blueprints/VirtualReality/BP_MotionController.BP_MotionController_C|GetRightGrabOrigin (Variables|Default|GetController))) _time) false false))))

(event EventOnGrab
  (|CallParentFunction))

(fn ConstructionScript)