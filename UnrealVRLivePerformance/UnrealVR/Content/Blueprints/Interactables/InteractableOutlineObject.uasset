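; An interactable object Blueprint that animates a two-part outline when selected or deselected, with an empty OnInteract event.
; Timelines drive the OutlineThickness material parameter on two components, Outline and Outline1.
; Selection animates Outline then Outline1 in sequence, and deselection runs separate timelines in reverse component order.
; Each event stops only one of the opposing pair of timelines before starting its own.
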(event EventBeginPlay)

(event Collision|EventActorBeginOverlap
  (params (OtherActor :type Actor%20Object%20Reference)))

(event EventTick
  (params (DeltaSeconds :type Float%20%28single-precision%29)))

(event EventOnInteract
  (params (controller :type Static%20Mesh%20Component%20Object%20Reference)))

(event EventOnSelected
  (Audio|Components|Audio|Stop (Variables|Default|GetHideOutline))
  (bind _time (Timeline|ShowOutline1 PlayFromStart)
    (:Update
      (Rendering|Material|SetScalarParameterValueonMaterials (Variables|Default|GetOutline) "OutlineThickness" _time))
    (:Finished
      (bind _time_2 (Timeline|ShowOutline PlayFromStart)
        (:Update
          (Rendering|Material|SetScalarParameterValueonMaterials (Variables|Default|GetOutline1) "OutlineThickness" _time_2))))))

(event EventOnDeselected
  (Audio|Components|Audio|Stop (Variables|Default|GetShowOutline))
  (bind _time (Timeline|HideOutline PlayFromStart)
    (:Update
      (Rendering|Material|SetScalarParameterValueonMaterials (Variables|Default|GetOutline1) "OutlineThickness" _time))
    (:Finished
      (bind _time_2 (Timeline|HideOutline1 PlayFromStart)
        (:Update
          (Rendering|Material|SetScalarParameterValueonMaterials (Variables|Default|GetOutline) "OutlineThickness" _time_2))))))

(fn ConstructionScript)