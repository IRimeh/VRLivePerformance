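; VR glow stick interactable that can be picked up with a motion controller and also serves as a tutorial trigger.
; On interact, physics turns off and a timeline pulls the mesh to the controller's right grab origin, restoring physics if nothing has attached it by the end.
; On release in TutorialMap, it sends step 3 to BP_TutorialController unless the tutorial is over.
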(event EventBeginPlay
  (bind _returnvalue (Game|GetCurrentLevelName true))
  (Variables|Default|SetisTutorial (Utilities|Enum|Equal(Enum) _returnvalue "TutorialMap")))

(event Collision|EventActorBeginOverlap
  (params (OtherActor :type Actor%20Object%20Reference)))

(event EventTick
  (params (DeltaSeconds :type Float%20%28single-precision%29)))

(event EventOnRelease
  (if (Variables|Default|GetisTutorial)
    (bind _outactors (Actor|GetAllActorsOfClass "/Game/Blueprints/Tutorial/BP_TutorialController.BP_TutorialController_C"))
    (if (not (Variables|/Game/Blueprints/Tutorial/BP_TutorialController.BP_TutorialController_C|GetIsTutorialOver (Utilities|Array|Get(acopy) _outactors)))
      (Default|EventNextStep (Utilities|Array|Get(acopy) _outactors) 3))))

(event EventOnInteract
  (params (controller :type Static%20Mesh%20Component%20Object%20Reference))
  (bind _asbp_motion_controller (Utilities|Casting|CastToBP_MotionController (Components|GetOwner controller)))
  (Variables|Default|SetController _asbp_motion_controller)
  (Physics|SetSimulatePhysics (Variables|Character|GetMesh) false)
  (bind _time (Timeline|Move%20To%20Controller PlayFromStart)
    (:Update
      (Transformation|SetWorldLocation (Variables|Character|GetMesh) (Math|Vector|Lerp(Vector) (Transformation|GetWorldLocation (Variables|Character|GetMesh)) (Transformation|GetWorldLocation (Variables|/Game/Blueprints/VirtualReality/BP_MotionController.BP_MotionController_C|GetRightGrabOrigin (Variables|Default|GetController))) _time) false false))
    (:Finished
      (if (not (Utilities|IsValid (Transformation|GetAttachParent (Variables|Character|GetMesh))))
        (Physics|SetSimulatePhysics (Variables|Character|GetMesh) true)))))

(fn ConstructionScript)