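; Left-side in-game menu actor that switches between Main, Objects, Settings and Emotes panels of overlap-triggered child-actor buttons.
; At BeginPlay it caches each panel's buttons; navigation toggles panel visibility and button overlap events, delaying activation after a switch.
; Tutorial support starts BP_TutorialController and opens menus with one active button highlighted by a pulsing material.
; Timeline-driven helpers fade text out, swap it and fade it back in.
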(event Custom|Enable%20Buttons
  (params (New%20Menu :type MenuOptionsEnum%20Enum :default "NewEnumerator0"))
  ;[1 1 1] Enables New Menu (Does Not Disable Old)
  (navigation|SetCurrentMenu New%20Menu)
  (Rendering|SetVisibility (Variables|Components|GetCurrentMenu) true true)
  (Utilities|FlowControl|Delay 1.0)
  (for _array_element (Variables|ButtonLists|GetCurrentMenuButtons)
    (if (!= (Variables|/Game/Blueprints/Menu/BP_ParentButton.BP_ParentButton_C|GetBox _array_element) 0)
      (Variables|/Script/Engine.PrimitiveComponent|SetbGenerateOverlapEvents (Variables|/Game/Blueprints/Menu/BP_ParentButton.BP_ParentButton_C|GetBox _array_element) true))))

(event Custom|Event%20TutorialNavigateToMenu
  (params (New%20Menu :type MenuOptionsEnum%20Enum :default "NewEnumerator0") (Button :type Child%20Actor%20Component%20Object%20Reference))
  ;[1 1 1] Navigate to new menu while enabling one pulsating button
  (bind _parentbutton (CallFunction|CastScenetoParentButton Button))
  (Navigation|DisableCurrentMenu)
  (navigation|SetCurrentMenu New%20Menu)
  (Rendering|SetVisibility (Variables|Components|GetCurrentMenu) true true)
  (if (!= (Variables|Default|GetPulsatingButtonCube) 0)
    (Rendering|Material|SetMaterial (Variables|Default|GetPulsatingButtonCube) 0 "/Game/Materials/VR/M_BaseMaterial.M_BaseMaterial"))
  (Utilities|FlowControl|Delay 2.0)
  (Variables|/Script/Engine.PrimitiveComponent|SetbGenerateOverlapEvents (Variables|/Game/Blueprints/Menu/BP_ParentButton.BP_ParentButton_C|GetBox _parentbutton) true)
  (Rendering|Material|SetMaterial (Variables|/Game/Blueprints/Menu/BP_ParentButton.BP_ParentButton_C|GetCube _parentbutton) 0 "/Game/Materials/Buttons/PulsingButton_M.PulsingButton_M")
  (Variables|Default|SetPulsatingButtonCube (Variables|/Game/Blueprints/Menu/BP_ParentButton.BP_ParentButton_C|GetCube _parentbutton)))

(event Custom|Event%20ChangeText
  (params (TextRender :type Text%20Render%20Component%20Object%20Reference) (NewText :type Text))
  ;[1 1 1] Fade in and out while changing it
  (bind _alpha (Timeline|Fade%20out PlayFromStart)
    (:Update
      (Rendering|Components|TextRender|SetTextRenderColor TextRender (Math|Conversions|ToColor(LinearColor) (Math|Color|MakeColor 0.0 0.0 0.0 _alpha))))
    (:Finished
      (Rendering|Components|TextRender|SetText TextRender NewText)
      (if (not (Utilities|Text|TextIsEmpty NewText))
        (bind _alpha_2 (Timeline|Fade%20in PlayFromStart)
          (:Update
            (Rendering|Components|TextRender|SetTextRenderColor TextRender (Math|Conversions|ToColor(LinearColor) (Math|Color|MakeColor 0.0 0.0 0.0 _alpha_2)))))))))

(event Custom|Event%20Delayed%20ChangeText
  (params (Text%20Render :type Text%20Render%20Component%20Object%20Reference) (New%20Text :type Text))
  (Utilities|FlowControl|Delay 2.0)
  (CallFunction|EventChangeText Text%20Render New%20Text))

(event Custom|Start%20Tutorial
  (bind _output_get (Variables|Default|SetisTutorial true))
  (if _output_get
    (Utilities|FlowControl|Delay 0.5)
    (bind _outactors (Actor|GetAllActorsOfClass "/Game/Blueprints/Tutorial/BP_TutorialController.BP_TutorialController_C"))
    (Default|EventNextStep (Utilities|Array|Get(acopy) _outactors))
    (else
      (CallFunction|EnableButtons "NewEnumerator0"))))

(event EventBeginPlay
  (CallFunction|SaveButtonsasVariable)
  (Variables|Components|SetCurrentMenu (Variables|Default|GetMainMenu))
  (CallFunction|EnableButtons "NewEnumerator0"))

(event Collision|EventActorBeginOverlap
  (params (OtherActor :type Actor%20Object%20Reference)))

(fn ConstructionScript)

(fn SaveButtonsasVariable
  ;[1 1 1] Add All Buttons To Their Respective Array
  (for _array_element (Components|GetChildrenComponents (Variables|Default|GetMainMenu) false)
    (bind _parentbutton (CallFunction|CastScenetoParentButton _array_element))
    (Utilities|Array|Add (Variables|ButtonLists|GetMainMenuButtons) _parentbutton))
  (for _array_element_2 (Components|GetChildrenComponents (Variables|Default|GetObjectsMenu) false)
    (bind _parentbutton_2 (CallFunction|CastScenetoParentButton _array_element_2))
    (Utilities|Array|Add (Variables|ButtonLists|GetObjectsButtons) _parentbutton_2))
  (for _array_element_3 (Components|GetChildrenComponents (Variables|Default|GetSettings) false)
    (bind _parentbutton_3 (CallFunction|CastScenetoParentButton _array_element_3))
    (Utilities|Array|Add (Variables|ButtonLists|GetSettingsButtons) _parentbutton_3))
  (for _array_element_4 (Components|GetChildrenComponents (Variables|Default|GetEmoteMenu) false)
    (bind _parentbutton_4 (CallFunction|CastScenetoParentButton _array_element_4))
    (Utilities|Array|Add (Variables|ButtonLists|GetEmoteButtons) _parentbutton_4))
  (return))

(fn CastScenetoParentButton
  (params (ButtonSceneComp :type Scene%20Component%20Object%20Reference))
  (bind _aschild_actor_component (Utilities|Casting|CastToChildActorComponent ButtonSceneComp))
  (bind _asbp_parent_button (Utilities|Casting|CastToBP_ParentButton (Variables|/Script/Engine.ChildActorComponent|GetChildActor _aschild_actor_component)))
  (return _asbp_parent_button))

(fn NavigatetoMenu
  (params (Menu%20Option :type MenuOptionsEnum%20Enum :default "NewEnumerator0"))
  (Navigation|DisableCurrentMenu)
  (CallFunction|EnableButtons Menu%20Option))

(fn DisableCurrentMenu
  (Rendering|SetVisibility (Variables|Components|GetCurrentMenu) false true)
  (for _array_element (Variables|ButtonLists|GetCurrentMenuButtons)
    (if (!= (Variables|/Game/Blueprints/Menu/BP_ParentButton.BP_ParentButton_C|GetBox _array_element) 0)
      (Variables|/Script/Engine.PrimitiveComponent|SetbGenerateOverlapEvents (Variables|/Game/Blueprints/Menu/BP_ParentButton.BP_ParentButton_C|GetBox _array_element) false)))
  (return))

(fn SetCurrentMenu
  (params (NewCurrentMenu :type MenuOptionsEnum%20Enum :default "NewEnumerator0"))
  (switch Utilities|FlowControl|Switch|SwitchonMenuOptionsEnum NewCurrentMenu
    (:NewEnumerator0
      (Variables|ButtonLists|SetCurrentMenuButtons (Variables|ButtonLists|GetMainMenuButtons))
      (Variables|Components|SetCurrentMenu (Variables|Default|GetMainMenu)))
    (:NewEnumerator1
      (Variables|ButtonLists|SetCurrentMenuButtons (Variables|ButtonLists|GetObjectsButtons))
      (Variables|Components|SetCurrentMenu (Variables|Default|GetObjectsMenu)))
    (:NewEnumerator2
      (Variables|ButtonLists|SetCurrentMenuButtons (Variables|ButtonLists|GetSettingsButtons))
      (Variables|Components|SetCurrentMenu (Variables|Default|GetSettings)))
    (:NewEnumerator3
      (Variables|ButtonLists|SetCurrentMenuButtons (Variables|ButtonLists|GetEmoteButtons))
      (Variables|Components|SetCurrentMenu (Variables|Default|GetEmoteMenu))))
  (return))

(fn DisableMenu
  (for _array_element (Variables|ButtonLists|GetCurrentMenuButtons)
    (if (!= (Variables|/Game/Blueprints/Menu/BP_ParentButton.BP_ParentButton_C|GetBox _array_element) 0)
      (Variables|/Script/Engine.PrimitiveComponent|SetbGenerateOverlapEvents (Variables|/Game/Blueprints/Menu/BP_ParentButton.BP_ParentButton_C|GetBox _array_element) false)))
  (return))

(fn EnableMenu
  (Navigation|NavigatetoMenu "NewEnumerator0")
  (return))

(fn DisablePulsatingButton
  (Rendering|Material|SetMaterial (Variables|Default|GetPulsatingButtonCube) 0 "/Game/Materials/VR/M_BaseMaterial.M_BaseMaterial"))