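; Settings menu button that raises or lowers Master, Music or SFX volume while pressed, depending on its direction flag.
; On BeginPlay an enum selects the sound class and menu percentage text.
; Tick adjusts the menu's stored volume within 0–100, updating the text and sound mix class override.
; Each press-action call increases the change speed, and release resets it.
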(event EventBeginPlay
  (|CallParentFunction)
  (CallFunction|SetAudioTypebyEnum))

(event Collision|EventActorBeginOverlap
  (params (OtherActor :type Actor%20Object%20Reference))
  (|CallParentFunction OtherActor) ; This node is disabled and will not be called.\nDrag off pins to build functionality.
)

(event EventTick
  (params (DeltaSeconds :type Float%20%28single-precision%29))
  (|CallParentFunction DeltaSeconds)
  (if (Variables|Default|GetButtonPressed)
    (CallFunction|ChangeVolume DeltaSeconds)))

(event EventResetButton)

(fn ConstructionScript
  (|CallParentFunction))

(fn PressButtonAction
  (Variables|Default|SetButtonPressed true)
  (Variables|Default|SetIncreaseSpeed (+ (Variables|Default|GetIncreaseSpeed) 0.1)))

(fn ReleaseButtonAction
  (Variables|Default|SetButtonPressed false)
  (Variables|Default|SetIncreaseSpeed 1.0))

(fn ChangeVolume
  (params (Delta%20Seconds :type Float%20%28single-precision%29))
  (bind _increasespeed (Variables|Default|GetIncreaseSpeed))
  (bind _audiotype (Variables|Default|GetAudioType))
  (bind _volumetextcomp (Variables|Default|GetVolumeTextComp))
  (bind _returnvalue (* Delta%20Seconds _increasespeed))
  (bind _volume (CallFunction|GetVolumebyAudioType))
  (if (Variables|Default|GetIncreaseVolume)
    (if (< _volume 1e+02)
      (CallFunction|SetVolumebyAudioType (Math|Float|Clamp(Float) (+ _volume _returnvalue) 0.0 1e+02))
      (Rendering|Components|TextRender|SetText _volumetextcomp (Utilities|Text|ToText(Integer) (Math|Float|Round (Math|Float|Clamp(Float) (+ _volume _returnvalue) 0.0 1e+02))))
      (Audio|SetSoundMixClassOverride "/Game/Audio/Classes/SoundMix.SoundMix" _audiotype (* (Math|Float|Clamp(Float) (+ _volume _returnvalue) 0.0 1e+02) 0.01) 1.0 0.0 true))
    (elif (> _volume 0.0)
      (CallFunction|SetVolumebyAudioType (Math|Float|Clamp(Float) (- _volume _returnvalue) 0.0 1e+02))
      (Rendering|Components|TextRender|SetText _volumetextcomp (Utilities|Text|ToText(Integer) (Math|Float|Round (Math|Float|Clamp(Float) (- _volume _returnvalue) 0.0 1e+02))))
      (Audio|SetSoundMixClassOverride "/Game/Audio/Classes/SoundMix.SoundMix" _audiotype (* (Math|Float|Clamp(Float) (- _volume _returnvalue) 0.0 1e+02) 0.01) 1.0 0.0 true))))

(fn SetAudioTypebyEnum
  (bind _menu (Variables|Default|GetMenu))
  (switch Utilities|FlowControl|Switch|SwitchonAudioTypeEnum (Variables|Default|GetAudioTypeEnum)
    (:NewEnumerator0
      (Variables|Default|SetAudioType "/Game/Audio/Classes/MasterAudio.MasterAudio")
      (Variables|Default|SetVolumeTextComp (Variables|/Game/Blueprints/Menu/Menus/BP_Menu_Left.BP_Menu_Left_C|GetMasterPerc _menu)))
    (:NewEnumerator1
      (Variables|Default|SetAudioType "/Game/Audio/Classes/MusicAudio.MusicAudio")
      (Variables|Default|SetVolumeTextComp (Variables|/Game/Blueprints/Menu/Menus/BP_Menu_Left.BP_Menu_Left_C|GetMusicPerc _menu)))
    (:NewEnumerator2
      (Variables|Default|SetAudioType "/Game/Audio/Classes/SFXAudio.SFXAudio")
      (Variables|Default|SetVolumeTextComp (Variables|/Game/Blueprints/Menu/Menus/BP_Menu_Left.BP_Menu_Left_C|GetSFXPerc _menu)))))

(fn GetVolumebyAudioType
  (bind _menu (Variables|Default|GetMenu))
  (switch Utilities|FlowControl|Switch|SwitchonAudioTypeEnum (Variables|Default|GetAudioTypeEnum)
    (:NewEnumerator0
      (return (Variables|/Game/Blueprints/Menu/Menus/BP_Menu_Left.BP_Menu_Left_C|GetMasterVolume _menu)))
    (:NewEnumerator1
      (return (Variables|/Game/Blueprints/Menu/Menus/BP_Menu_Left.BP_Menu_Left_C|GetMusicVolume _menu)))
    (:NewEnumerator2
      (return (Variables|/Game/Blueprints/Menu/Menus/BP_Menu_Left.BP_Menu_Left_C|GetSFXVolume _menu)))))

(fn SetVolumebyAudioType
  (params (New%20Volume :type Float%20%28single-precision%29))
  (bind _menu (Variables|Default|GetMenu))
  (switch Utilities|FlowControl|Switch|SwitchonAudioTypeEnum (Variables|Default|GetAudioTypeEnum)
    (:NewEnumerator0
      (Variables|/Game/Blueprints/Menu/Menus/BP_Menu_Left.BP_Menu_Left_C|SetMasterVolume _menu New%20Volume))
    (:NewEnumerator1
      (Variables|/Game/Blueprints/Menu/Menus/BP_Menu_Left.BP_Menu_Left_C|SetMusicVolume _menu New%20Volume))
    (:NewEnumerator2
      (Variables|/Game/Blueprints/Menu/Menus/BP_Menu_Left.BP_Menu_Left_C|SetSFXVolume _menu New%20Volume))))