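; Parent actor for menu buttons that spawn an object into the player's right VR controller hand when pressed.
; The construction script picks the button's icon material from the Icon setting.
; PressButtonAction looks up and stores the right controller through the game instance if needed, also spawning a lighter in the left hand for fireworks.
; With IsTutorial set, a press also advances an unfinished tutorial.
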(event EventBeginPlay
  (|CallParentFunction))

(event Collision|EventActorBeginOverlap
  (params (OtherActor :type Actor%20Object%20Reference))
  (|CallParentFunction OtherActor) ; This node is disabled and will not be called.\nDrag off pins to build functionality.
)

(event EventTick
  (params (DeltaSeconds :type Float%20%28single-precision%29))
  (|CallParentFunction DeltaSeconds) ; This node is disabled and will not be called.\nDrag off pins to build functionality.
)

(fn ConstructionScript
  (bind _buttonicon (Variables|Default|GetButtonIcon))
  (switch int (Variables|Default|GetIcon)
    (:Default
      (Rendering|Material|SetMaterial _buttonicon 0 "/Game/Materials/Menu/Interactables/Mat_Glowstick.Mat_Glowstick" :!label _label))
    (:0
      (goto _label))
    (:1
      (Rendering|Material|SetMaterial _buttonicon 0 "/Game/Materials/Menu/Interactables/Mat_LightOrb.Mat_LightOrb"))
    (:2
      (Rendering|Material|SetMaterial _buttonicon 0 "/Game/Materials/Menu/Interactables/Mat_CameraButton.Mat_CameraButton"))
    (:3
      (Rendering|Material|SetMaterial _buttonicon 0 "/Game/Materials/Menu/Interactables/Mat_Lighter.Mat_Lighter"))
    (:4
      (Rendering|Material|SetMaterial _buttonicon 0 "/Game/Materials/Menu/Interactables/Mat_Firework.Mat_Firework"))))

(fn PressButtonAction
  (if (== (Variables|Default|GetObjectBP) "/Game/Blueprints/Interactables/Firework.Firework_C")
    (CallFunction|SpawnLighterLeft))
  (if (Utilities|IsValid (Variables|Default|GetRightController))
    _
    (else
      (bind _ascustom_game_instance (Utilities|Casting|CastToCustomGameInstance (Game|GetGameInstance)))
      (Variables|Default|SetRightController (Variables|/Game/Blueprints/Player/VRPawn.VRPawn_C|GetRightController (Variables|/Game/Blueprints/ProjectSettings/CustomGameInstance.CustomGameInstance_C|GetPlayer _ascustom_game_instance)))))
  (Default|SpawnObjectinHand (Variables|Default|GetRightController) (Variables|Default|GetObjectBP) false "0, 0, 0")
  (if (Variables|Default|GetisTutorial)
    (bind _outactors (Actor|GetAllActorsOfClass "/Game/Blueprints/Tutorial/BP_TutorialController.BP_TutorialController_C"))
    (if (not (Variables|/Game/Blueprints/Tutorial/BP_TutorialController.BP_TutorialController_C|GetIsTutorialOver (Utilities|Array|Get(acopy) _outactors)))
      (Default|EventNextStep (Utilities|Array|Get(acopy) _outactors) 2))))

(fn SpawnLighterLeft
  (bind _ascustom_game_instance (Utilities|Casting|CastToCustomGameInstance (Game|GetGameInstance)))
  (Default|SpawnObjectinHand (Variables|/Game/Blueprints/Player/VRPawn.VRPawn_C|GetLeftController (Variables|/Game/Blueprints/ProjectSettings/CustomGameInstance.CustomGameInstance_C|GetPlayer _ascustom_game_instance)) "/Game/Blueprints/Interactables/Lighter.Lighter_C" false "0, 0, 0"))