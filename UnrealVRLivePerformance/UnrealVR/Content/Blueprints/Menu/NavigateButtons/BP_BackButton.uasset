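; BP_BackButton is a menu navigation button that sends the menu to a fixed destination when pressed.
; It overrides PressButtonAction, calling NavigateToMenu on its Menu reference when outside the tutorial or once the tutorial is over.
; During an unfinished tutorial, it instead passes its Step to the first BP_TutorialController found in the level through EventNextStep, so the press advances the tutorial without navigating.
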(event EventBeginPlay
  (|CallParentFunction))

(event Collision|EventActorBeginOverlap
  (params (OtherActor :type Actor%20Object%20Reference))
  (|CallParentFunction OtherActor) ; This node is disabled and will not be called.\nDrag off pins to build functionality.
)

(event EventTick
  (params (DeltaSeconds :type Float%20%28single-precision%29))
  (|CallParentFunction DeltaSeconds) ; This node is disabled and will not be called.\nDrag off pins to build functionality.
)

(fn ConstructionScript
  (|CallParentFunction))

(fn PressButtonAction
  (if (Variables|Default|GetisTutorial)
    (bind _outactors (Actor|GetAllActorsOfClass "/Game/Blueprints/Tutorial/BP_TutorialController.BP_TutorialController_C"))
    (if (Variables|/Game/Blueprints/Tutorial/BP_TutorialController.BP_TutorialController_C|GetIsTutorialOver (Utilities|Array|Get(acopy) _outactors))
      (Default|NavigatetoMenu (Variables|Default|GetMenu) "NewEnumerator0" :!label _label)
      (else
        (Default|EventNextStep (Utilities|Array|Get(acopy) _outactors) (Variables|Default|GetStep))))
    (else
      (goto _label))))