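; BP_BackButton is a navigation button actor that returns the menu to a fixed page or advances the tutorial.
; Its logic lives in PressButtonAction, which normally calls NavigateToMenu on Menu with the first enum entry.
; When IsTutorial is set, each press instead increments Step, and the first two presses send hard-coded step numbers to the first BP_TutorialController found in the level.
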(event EventBeginPlay
  (|CallParentFunction) ; This node is disabled and will not be called.\nDrag off pins to build functionality.
)

(event Collision|EventActorBeginOverlap
  (params (OtherActor :type Actor%20Object%20Reference))
  (|CallParentFunction OtherActor) ; This node is disabled and will not be called.\nDrag off pins to build functionality.
)

(event EventTick
  (params (DeltaSeconds :type Float%20%28single-precision%29))
  (|CallParentFunction DeltaSeconds) ; This node is disabled and will not be called.\nDrag off pins to build functionality.
)

(fn ConstructionScript
  (|CallParentFunction))

(fn PressButtonAction
  (if (Variables|Default|GetisTutorial)
    (bind _output_get (Variables|Default|SetStep (+ (Variables|Default|GetStep) 1)))
    (bind _outactors (Actor|GetAllActorsOfClass "/Game/Blueprints/Tutorial/BP_TutorialController.BP_TutorialController_C"))
    (switch int _output_get
      (:1
        (Default|EventNextStep (Utilities|Array|Get(acopy) _outactors) 4))
      (:2
        (Default|EventNextStep (Utilities|Array|Get(acopy) _outactors) 6)))
    (else
      (Default|NavigatetoMenu (Variables|Default|GetMenu) "NewEnumerator0"))))