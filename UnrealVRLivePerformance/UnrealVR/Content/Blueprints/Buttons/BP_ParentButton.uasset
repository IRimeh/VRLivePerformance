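; Base VR push button with a construction-script text label, pressed by a BP_MotionController fingertip.
; Fingertip overlap locks out new presses and opens a Tick-driven gate that slides the cube along local Z with the finger, clamped to PressDistance.
; Full depth calls ButtonAction, an empty hook, then resets.
; Reset, also triggered when the controller's GrabSphere exits, closes the gate and timeline-lerps the cube back before re-enabling presses.
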(event OnComponentBeginOverlap(Box)
  (params (OverlappedComponent :type Primitive%20Component%20Object%20Reference) (OtherActor :type Actor%20Object%20Reference) (OtherComp :type Primitive%20Component%20Object%20Reference) (OtherBodyIndex :type Integer) (bFromSweep :type Boolean) (SweepResult :type Hit%20Result%20Structure%20%28by%20ref%29))
  ;[1 1 1] Get button
  (if (not (Variables|Default|GetDisablePress))
    (bind _asbp_motion_controller (Utilities|Casting|CastToBP_MotionController OtherActor))
    (if (== (Variables|/Game/Blueprints/VirtualRealityBP/Blueprints/BP_MotionController.BP_MotionController_C|GetFingerTip _asbp_motion_controller) OtherComp)
      (Variables|Default|SetDisablePress true)
      (Variables|Default|SetFingerTip (Variables|/Game/Blueprints/VirtualRealityBP/Blueprints/BP_MotionController.BP_MotionController_C|GetFingerTip _asbp_motion_controller))
      (Variables|Default|SetButtonStartLocation (Variables|/Script/Engine.SceneComponent|GetRelativeLocation (Variables|Default|GetCube)))
      ;[1 1 1] Calculate location
      (Utilities|FlowControl|Gate true) ; enters at Open
    )))

(event OnComponentEndOverlap(Box)
  (params (OverlappedComponent :type Primitive%20Component%20Object%20Reference) (OtherActor :type Actor%20Object%20Reference) (OtherComp :type Primitive%20Component%20Object%20Reference) (OtherBodyIndex :type Integer))
  (bind _returnvalue (Transformation|GetActorTransform))
  (bind _fingertip (Variables|Default|GetFingerTip))
  (bind _buttonstartlocation (Variables|Default|GetButtonStartLocation))
  (bind _buttonstartlocation_2 (Variables|Default|GetButtonStartLocation))
  (bind _buttonstartlocation_3 (Variables|Default|GetButtonStartLocation))
  (bind _returnvalue_2 (Transformation|GetWorldLocation _fingertip))
  (bind _z (Math|Vector|BreakVector _buttonstartlocation_2))
  (bind (_x _y _z_2) (Math|Vector|BreakVector _buttonstartlocation_3))
  (bind _returnvalue_3 (Math|Transform|InverseTransformLocation _returnvalue _returnvalue_2))
  (bind _returnvalue_4 (- _returnvalue_3 _buttonstartlocation))
  (bind _z_3 (Math|Vector|BreakVector _returnvalue_4))
  (bind _returnvalue_5 (Math|Vector|MakeVector 0.0 0.0 _z_3))
  (bind _returnvalue_6 (+ _buttonstartlocation_2 _returnvalue_5))
  (bind (_x_2 _y_2 _z_4) (Math|Vector|BreakVector _returnvalue_6))
  ;[1 1 1] Returning button to orginal location
  (bind _asbp_motion_controller (Utilities|Casting|CastToBP_MotionController OtherActor))
  (if (== (Variables|/Game/VirtualRealityBP/Blueprints/BP_MotionController.BP_MotionController_C|GetGrabSphere _asbp_motion_controller) OtherComp)
    (Utilities|FlowControl|Sequence
      (:then_0
        ;[1 1 1] Calculate location
        (Utilities|FlowControl|Gate true) ; enters at Close
      )
      (:then_1
        (bind _driver (Timeline|SnapBack%20Timeline PlayFromStart)
          (:Update
            (Transformation|SetRelativeLocation (Variables|Default|GetCube) (Math|Vector|MakeVector _x _y (Math|Float|Lerp (.Z (Math|Vector|BreakVector (Variables|/Script/Engine.SceneComponent|GetRelativeLocation (Variables|Default|GetCube)))) _z_2 _driver)) false false))
          (:Finished
            (Variables|Default|SetDisablePress false)))))))

(event Custom|ResetButton
  (bind _returnvalue (Transformation|GetActorTransform))
  (bind _fingertip (Variables|Default|GetFingerTip))
  (bind _buttonstartlocation (Variables|Default|GetButtonStartLocation))
  (bind _buttonstartlocation_2 (Variables|Default|GetButtonStartLocation))
  (bind _buttonstartlocation_3 (Variables|Default|GetButtonStartLocation))
  (bind _returnvalue_2 (Transformation|GetWorldLocation _fingertip))
  (bind _z (Math|Vector|BreakVector _buttonstartlocation_2))
  (bind (_x _y _z_2) (Math|Vector|BreakVector _buttonstartlocation_3))
  (bind _returnvalue_3 (Math|Transform|InverseTransformLocation _returnvalue _returnvalue_2))
  (bind _returnvalue_4 (- _returnvalue_3 _buttonstartlocation))
  (bind _z_3 (Math|Vector|BreakVector _returnvalue_4))
  (bind _returnvalue_5 (Math|Vector|MakeVector 0.0 0.0 _z_3))
  (bind _returnvalue_6 (+ _buttonstartlocation_2 _returnvalue_5))
  (bind (_x_2 _y_2 _z_4) (Math|Vector|BreakVector _returnvalue_6))
  ;[1 1 1] Returning button to orginal location
  (Utilities|FlowControl|Sequence
    (:then_0
      ;[1 1 1] Calculate location
      (Utilities|FlowControl|Gate true) ; enters at Close
    )
    (:then_1
      (bind _driver (Timeline|SnapBack%20Timeline PlayFromStart)
        (:Update
          (Transformation|SetRelativeLocation (Variables|Default|GetCube) (Math|Vector|MakeVector _x _y (Math|Float|Lerp (.Z (Math|Vector|BreakVector (Variables|/Script/Engine.SceneComponent|GetRelativeLocation (Variables|Default|GetCube)))) _z_2 _driver)) false false))
        (:Finished
          (Variables|Default|SetDisablePress false))))))

(event EventBeginPlay)

(event Collision|EventActorBeginOverlap
  (params (OtherActor :type Actor%20Object%20Reference)))

(event EventTick
  (params (DeltaSeconds :type Float%20%28single-precision%29))
  (bind _returnvalue (Transformation|GetActorTransform))
  (bind _fingertip (Variables|Default|GetFingerTip))
  (bind _buttonstartlocation (Variables|Default|GetButtonStartLocation))
  (bind _buttonstartlocation_2 (Variables|Default|GetButtonStartLocation))
  (bind _returnvalue_2 (Transformation|GetWorldLocation _fingertip))
  (bind _z (Math|Vector|BreakVector _buttonstartlocation_2))
  (bind _returnvalue_3 (Math|Transform|InverseTransformLocation _returnvalue _returnvalue_2))
  (bind _returnvalue_4 (- _returnvalue_3 _buttonstartlocation))
  (bind _z_2 (Math|Vector|BreakVector _returnvalue_4))
  (bind _returnvalue_5 (Math|Vector|MakeVector 0.0 0.0 _z_2))
  (bind _returnvalue_6 (+ _buttonstartlocation_2 _returnvalue_5))
  (bind (_x _y _z_3) (Math|Vector|BreakVector _returnvalue_6))
  ;[1 1 1] Calculate location
  (Utilities|FlowControl|Gate true
    (:Exit
      (Transformation|SetRelativeLocation (Variables|Default|GetCube) (Math|Vector|MakeVector _x _y (Math|Float|Clamp(Float) _z_3 (- _z (Variables|Default|GetPressDistance)) _z)) false false)
      ;[1 1 1] Press button
      (if (Math|Float|NearlyEqual(Float) (.Z (Math|Vector|BreakVector (Variables|/Script/Engine.SceneComponent|GetRelativeLocation (Variables|Default|GetCube)))) (- (.Z (Math|Vector|BreakVector (Variables|Default|GetButtonStartLocation))) (Variables|Default|GetPressDistance)) 0.1)
        (CallFunction|ButtonAction)
        (CallFunction|ResetButton)))))

(fn ConstructionScript
  ;[1 1 1] Setting the text
  (Rendering|Components|TextRender|SetText (Variables|Default|GetTextRenderer) (Variables|Default|GetButtonText)))

(fn ButtonAction)