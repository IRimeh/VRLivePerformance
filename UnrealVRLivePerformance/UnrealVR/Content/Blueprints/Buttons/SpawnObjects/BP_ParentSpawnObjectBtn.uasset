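; Base Blueprint for buttons that spawn an object into the player's right hand when pressed.
; PressButtonAction gets the right controller from the player in CustomGameInstance if not already valid, then tells it to spawn ObjectBP in hand without custom rotation.
; When IsTutorial is set, the press also advances the first BP_TutorialController found via EventNextStep.
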(event EventBeginPlay
  (|CallParentFunction))

(event Collision|EventActorBeginOverlap
  (params (OtherActor :type Actor%20Object%20Reference))
  (|CallParentFunction OtherActor) ; This node is disabled and will not be called.\nDrag off pins to build functionality.
)

(event EventTick
  (params (DeltaSeconds :type Float%20%28single-precision%29))
  (|CallParentFunction DeltaSeconds) ; This node is disabled and will not be called.\nDrag off pins to build functionality.
)

(fn ConstructionScript)

(fn PressButtonAction
  (if (Utilities|IsValid (Variables|Default|GetRightController))
    _
    (else
      (bind _ascustom_game_instance (Utilities|Casting|CastToCustomGameInstance (Game|GetGameInstance)))
      (Variables|Default|SetRightController (Variables|/Game/Blueprints/Player/VRPawn.VRPawn_C|GetRightController (Variables|/Game/Blueprints/ProjectSettings/CustomGameInstance.CustomGameInstance_C|GetPlayer _ascustom_game_instance)))))
  (Default|SpawnObjectinHand (Variables|Default|GetRightController) (Variables|Default|GetObjectBP) false "0, 0, 0")
  (if (Variables|Default|GetisTutorial)
    (bind _outactors (Actor|GetAllActorsOfClass "/Game/Blueprints/Tutorial/BP_TutorialController.BP_TutorialController_C"))
    (Default|EventNextStep (Utilities|Array|Get(acopy) _outactors) 2)))