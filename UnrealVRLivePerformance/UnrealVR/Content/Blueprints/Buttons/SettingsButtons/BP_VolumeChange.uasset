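; BP_VolumeChange is a settings button that raises or lowers the master audio volume while pressed, with direction set by IncreaseVolume.
; Press and release actions toggle ButtonPressed; each press call bumps IncreaseSpeed and release resets it.
; While pressed, Tick runs ChangeVolume, stepping the Menu's clamped percentage by delta time and speed.
; Each step updates the Menu's rounded readout and applies a SoundMix class override to MasterAudio.
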(event EventBeginPlay
  (|CallParentFunction))

(event Collision|EventActorBeginOverlap
  (params (OtherActor :type Actor%20Object%20Reference))
  (|CallParentFunction OtherActor) ; This node is disabled and will not be called.\nDrag off pins to build functionality.
)

(event EventTick
  (params (DeltaSeconds :type Float%20%28single-precision%29))
  (|CallParentFunction DeltaSeconds)
  (if (Variables|Default|GetButtonPressed)
    (CallFunction|ChangeVolume DeltaSeconds)))

(event EventResetButton)

(fn ConstructionScript
  (|CallParentFunction))

(fn PressButtonAction
  (Variables|Default|SetButtonPressed true)
  (Variables|Default|SetIncreaseSpeed (+ (Variables|Default|GetIncreaseSpeed) 0.1)))

(fn ReleaseButtonAction
  (Variables|Default|SetButtonPressed false)
  (Variables|Default|SetIncreaseSpeed 1.0))

(fn ChangeVolume
  (params (Delta%20Seconds :type Float%20%28single-precision%29))
  (bind _increasespeed (Variables|Default|GetIncreaseSpeed))
  (bind _menu (Variables|Default|GetMenu))
  (bind _menu_2 (Variables|Default|GetMenu))
  (bind _returnvalue (* Delta%20Seconds _increasespeed))
  (bind _volumeper (Variables|/Game/Blueprints/Buttons/Menus/BP_Menu_Left.BP_Menu_Left_C|GetVolumePer _menu))
  (if (Variables|Default|GetIncreaseVolume)
    (if (< (Variables|/Game/Blueprints/Buttons/Menus/BP_Menu_Left.BP_Menu_Left_C|GetVolumePercentage _menu_2) 1e+02)
      (bind _output_get (Variables|/Game/Blueprints/Buttons/Menus/BP_Menu_Left.BP_Menu_Left_C|SetVolumePercentage _menu_2 (Math|Float|Clamp(Float) (+ (Variables|/Game/Blueprints/Buttons/Menus/BP_Menu_Left.BP_Menu_Left_C|GetVolumePercentage _menu_2) _returnvalue) 0.0 1e+02)))
      (Rendering|Components|TextRender|SetText _volumeper (Utilities|Text|ToText(Integer) (Math|Float|Round _output_get)))
      (Audio|SetSoundMixClassOverride "/Game/Audio/Classes/SoundMix.SoundMix" "/Game/Audio/Classes/MasterAudio.MasterAudio" (* (Variables|/Game/Blueprints/Buttons/Menus/BP_Menu_Left.BP_Menu_Left_C|GetVolumePercentage _menu) 0.01) 1.0 0.0 true))
    (elif (> (Variables|/Game/Blueprints/Buttons/Menus/BP_Menu_Left.BP_Menu_Left_C|GetVolumePercentage _menu_2) 0.0)
      (bind _output_get_2 (Variables|/Game/Blueprints/Buttons/Menus/BP_Menu_Left.BP_Menu_Left_C|SetVolumePercentage _menu_2 (Math|Float|Clamp(Float) (- (Variables|/Game/Blueprints/Buttons/Menus/BP_Menu_Left.BP_Menu_Left_C|GetVolumePercentage _menu_2) _returnvalue) 0.0 1e+02)))
      (Rendering|Components|TextRender|SetText _volumeper (Utilities|Text|ToText(Integer) (Math|Float|Round _output_get_2)))
      (Audio|SetSoundMixClassOverride "/Game/Audio/Classes/SoundMix.SoundMix" "/Game/Audio/Classes/MasterAudio.MasterAudio" (* (Variables|/Game/Blueprints/Buttons/Menus/BP_Menu_Left.BP_Menu_Left_C|GetVolumePercentage _menu) 0.01) 1.0 0.0 true))))