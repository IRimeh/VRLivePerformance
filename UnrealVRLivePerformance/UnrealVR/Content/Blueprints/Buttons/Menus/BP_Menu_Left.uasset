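; Left menu actor that switches between Main, Objects and Settings panels of overlap-triggered child-actor buttons.
; BeginPlay caches each panel's BP_ParentButton children; navigation toggles panel visibility and button overlap events, delaying activation by one second.
; On TutorialMap, it enables only the specified button and highlights it with a pulsing material, restoring the previous one.
; ChangeText uses fade timelines to swap text render content.
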(event Custom|Enable%20Buttons
  (params (New%20Menu :type MenuOptionsEnum%20Enum :default "NewEnumerator0"))
  ;[1 1 1] Enables New Menu (Does Not Disable Old)
  (navigation|SetCurrentMenu New%20Menu)
  (Rendering|SetVisibility (Variables|Components|GetCurrentMenu) true true)
  (Utilities|FlowControl|Delay 1.0)
  (for _array_element (Variables|ButtonLists|GetCurrentMenuButtons)
    (Variables|/Script/Engine.PrimitiveComponent|SetbGenerateOverlapEvents (Variables|/Game/Blueprints/Buttons/BP_ParentButton.BP_ParentButton_C|GetBox _array_element) true)))

(event Custom|Event%20ChangeText
  (params (TextRender :type Text%20Render%20Component%20Object%20Reference) (NewText :type Text))
  ;[1 1 1] Fade in and out while changing it
  (bind _alpha (Timeline|Fade%20out Play)
    (:Update
      (Rendering|Components|TextRender|SetTextRenderColor TextRender (Math|Conversions|ToColor(LinearColor) (Math|Color|MakeColor 255.0 255.0 255.0 _alpha)))
      (Rendering|Components|TextRender|SetText TextRender NewText)
      (if (not (Utilities|Text|TextIsEmpty NewText))
        (bind _alpha_2 (Timeline|Fade%20in Play)
          (:Update
            (Rendering|Components|TextRender|SetTextRenderColor TextRender (Math|Conversions|ToColor(LinearColor) (Math|Color|MakeColor 255.0 255.0 255.0 _alpha_2)))))))))

(event EventBeginPlay
  (bind _returnvalue (Game|GetCurrentLevelName true))
  (bind _output_get (Variables|Default|SetisTutorial (Utilities|Enum|Equal(Enum) _returnvalue "TutorialMap")))
  (CallFunction|SaveButtonsasVariable)
  (Variables|Components|SetCurrentMenu (Variables|Default|GetMainMenu))
  (if _output_get
    (Tutorial|TutorialNavigatetoMenu "NewEnumerator0" (Variables|Default|GetObjectsMenuButton))
    (else
      (CallFunction|EnableButtons "NewEnumerator0"))))

(event Collision|EventActorBeginOverlap
  (params (OtherActor :type Actor%20Object%20Reference)))

(fn ConstructionScript)

(fn SaveButtonsasVariable
  ;[1 1 1] Add All Buttons To Their Respective Array
  (for _array_element (Components|GetChildrenComponents (Variables|Default|GetMainMenu) false)
    (bind _parentbutton (CallFunction|CastScenetoParentButton _array_element))
    (Utilities|Array|Add (Variables|ButtonLists|GetMainMenuButtons) _parentbutton))
  (for _array_element_2 (Components|GetChildrenComponents (Variables|Default|GetObjectsMenu) false)
    (bind _parentbutton_2 (CallFunction|CastScenetoParentButton _array_element_2))
    (Utilities|Array|Add (Variables|ButtonLists|GetObjectsButtons) _parentbutton_2))
  (for _array_element_3 (Components|GetChildrenComponents (Variables|Default|GetSettings) false)
    (bind _parentbutton_3 (CallFunction|CastScenetoParentButton _array_element_3))
    (Utilities|Array|Add (Variables|ButtonLists|GetSettingsButtons) _parentbutton_3))
  (return))

(fn CastScenetoParentButton
  (params (ButtonSceneComp :type Scene%20Component%20Object%20Reference))
  (bind _aschild_actor_component (Utilities|Casting|CastToChildActorComponent ButtonSceneComp))
  (bind _asbp_parent_button (Utilities|Casting|CastToBP_ParentButton (Variables|/Script/Engine.ChildActorComponent|GetChildActor _aschild_actor_component)))
  (return _asbp_parent_button))

(fn NavigatetoMenu
  (params (Menu%20Option :type MenuOptionsEnum%20Enum :default "NewEnumerator0"))
  (Navigation|DisableCurrentMenu)
  (CallFunction|EnableButtons Menu%20Option))

(fn DisableCurrentMenu
  (Rendering|SetVisibility (Variables|Components|GetCurrentMenu) false true)
  (for _array_element (Variables|ButtonLists|GetCurrentMenuButtons)
    (Variables|/Script/Engine.PrimitiveComponent|SetbGenerateOverlapEvents (Variables|/Game/Blueprints/Buttons/BP_ParentButton.BP_ParentButton_C|GetBox _array_element) false))
  (return))

(fn SetCurrentMenu
  (params (NewCurrentMenu :type MenuOptionsEnum%20Enum :default "NewEnumerator0"))
  (switch Utilities|FlowControl|Switch|SwitchonMenuOptionsEnum NewCurrentMenu
    (:NewEnumerator0
      (Variables|ButtonLists|SetCurrentMenuButtons (Variables|ButtonLists|GetMainMenuButtons))
      (Variables|Components|SetCurrentMenu (Variables|Default|GetMainMenu)))
    (:NewEnumerator1
      (Variables|ButtonLists|SetCurrentMenuButtons (Variables|ButtonLists|GetObjectsButtons))
      (Variables|Components|SetCurrentMenu (Variables|Default|GetObjectsMenu)))
    (:NewEnumerator2
      (Variables|ButtonLists|SetCurrentMenuButtons (Variables|ButtonLists|GetSettingsButtons))
      (Variables|Components|SetCurrentMenu (Variables|Default|GetSettings))))
  (return))

(fn DisableMenu
  (for _array_element (Variables|ButtonLists|GetCurrentMenuButtons)
    (Variables|/Script/Engine.PrimitiveComponent|SetbGenerateOverlapEvents (Variables|/Game/Blueprints/Buttons/BP_ParentButton.BP_ParentButton_C|GetBox _array_element) false))
  (return))

(fn EnableMenu
  (Navigation|NavigatetoMenu "NewEnumerator0")
  (return))

(fn TutorialNavigatetoMenu
  (params (New%20Menu :type MenuOptionsEnum%20Enum :default "NewEnumerator0") (Button :type Child%20Actor%20Component%20Object%20Reference))
  (bind _parentbutton (CallFunction|CastScenetoParentButton Button))
  (navigation|SetCurrentMenu New%20Menu)
  (Rendering|SetVisibility (Variables|Components|GetCurrentMenu) true true)
  (Variables|/Script/Engine.PrimitiveComponent|SetbGenerateOverlapEvents (Variables|/Game/Blueprints/Buttons/BP_ParentButton.BP_ParentButton_C|GetBox _parentbutton) true)
  (Rendering|Material|SetMaterial (Variables|/Game/Blueprints/Buttons/BP_ParentButton.BP_ParentButton_C|GetCube _parentbutton) 0 "/Game/Materials/Buttons/PulsingButton_M.PulsingButton_M")
  (if (!= (Variables|Default|GetPulsatingButtonCube) 0)
    (Rendering|Material|SetMaterial (Variables|Default|GetPulsatingButtonCube) 0 "/Game/Materials/VR/M_BaseMaterial.M_BaseMaterial"))
  (Variables|Default|SetPulsatingButtonCube (Variables|/Game/Blueprints/Buttons/BP_ParentButton.BP_ParentButton_C|GetCube _parentbutton)))